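; AC_HealthComponent is a shared player component that tracks health, starting at MaxHealth on BeginPlay.
; TakeDamage subtracts damage, then calls OnDamageTaken while health stays above zero or OnDeath otherwise.
; Heal adds the Healing variable, clamps overflow to MaxHealth and calls OnHeal.
; Its CheckIfFullHealth guard uses a strict greater-than, so healing at exactly full health still calls OnHeal.
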(event Custom|TakeDamage
  (params (Damage :type Float%20%28double-precision%29))
  (bind _output_get (Variables|Default|SetCurrentHealth (- (Variables|Default|GetCurrentHealth) Damage)))
  (if (> _output_get 0.0)
    (Default|CallOnDamageTaken)
    (else
      (Default|CallOnDeath))))

(event Custom|Heal
  (bind _fullhealth_ (CallFunction|CheckifFullHealth))
  (if (not _fullhealth_)
    (Variables|Default|SetCurrentHealth (+ (Variables|Default|GetCurrentHealth) (Variables|Default|GetHealing)))
    (bind _fullhealth__2 (CallFunction|CheckifFullHealth))
    (if _fullhealth__2
      (Variables|Default|SetCurrentHealth (Variables|Default|GetMaxHealth)))
    (Default|CallOnHeal)))

(event EventBeginPlay
  (Variables|Default|SetCurrentHealth (Variables|Default|GetMaxHealth)))

(fn CheckifFullHealth
  (return (> (Variables|Default|GetCurrentHealth) (Variables|Default|GetMaxHealth))))