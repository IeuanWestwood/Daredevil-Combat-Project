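; Actor component that shows floating health and posture bars above its owning actor.
; On BeginPlay it adds two world-space widget components at staggered heights, each hosting its own bar widget.
; It binds to the owner's AC_HealthComponent damage, death and stun-end events to refresh both bars.
; Each tick it turns visible bars toward the player camera on yaw only, as a simple billboard.
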(event Custom|UpdateHealthAndPosture
  (bind _healthcomponent (Variables|Default|GetHealthComponent))
  (bind _healthcomponent_2 (Variables|Default|GetHealthComponent))
  (Default|HealthUpdated (Variables|Default|GetHealthBarWidget) (Variables|/Game/MainContent/Design/Player/SharedComponents/AC_HealthComponent.AC_HealthComponent_C|GetMaxHealth _healthcomponent_2) (Variables|/Game/MainContent/Design/Player/SharedComponents/AC_HealthComponent.AC_HealthComponent_C|GetCurrentHealth _healthcomponent_2))
  (Default|PostureUpdated (Variables|Default|GetPostureBarWidget) (Variables|/Game/MainContent/Design/Player/SharedComponents/AC_HealthComponent.AC_HealthComponent_C|GetPostureThreshold _healthcomponent) (Variables|/Game/MainContent/Design/Player/SharedComponents/AC_HealthComponent.AC_HealthComponent_C|GetCurrentPosture _healthcomponent)))

(event EventBeginPlay
  (Variables|Default|SetPlayerCamera (Game|GetPlayerCameraManager 0))
  (Utilities|FlowControl|Sequence
    (:then_0
      (bind _returnvalue (Game|AddComponentbyClass (Components|GetOwner) "/Script/UMG.WidgetComponent" false (Math|Transform|MakeTransform (Math|Vector|MakeVector 0.0 0.0 (Variables|Default|GetOverheadDistance)) "0, 0, 0" "1.000000,1.000000,1.000000")))
      (bind _output_get (Variables|Default|SetHealthbarComponent _returnvalue))
      (Class|WidgetComponent|SetDrawatDesiredSize _output_get true)
      (Class|WidgetComponent|SetWidgetSpace _output_get "World")
      (bind _returnvalue_2 (UserInterface|CreateWidget "/Game/MainContent/Design/UI/WBP_OverHeadHealth.WBP_OverHeadHealth_C"))
      (bind _output_get_2 (Variables|Default|SetHealthBarWidget _returnvalue_2))
      (UserInterface|SetWidget (Variables|Default|GetHealthbarComponent) _output_get_2))
    (:then_1
      (bind _returnvalue_3 (Game|AddComponentbyClass (Components|GetOwner) "/Script/UMG.WidgetComponent" false (Math|Transform|MakeTransform (Math|Vector|MakeVector 0.0 0.0 (* (Variables|Default|GetOverheadDistance) 1.5)) "0, 0, 0" "1.000000,1.000000,1.000000")))
      (bind _output_get_3 (Variables|Default|SetPosturebarComponent _returnvalue_3))
      (Class|WidgetComponent|SetDrawatDesiredSize _output_get_3 true)
      (Class|WidgetComponent|SetWidgetSpace _output_get_3 "World")
      (bind _returnvalue_4 (UserInterface|CreateWidget "/Game/MainContent/Design/UI/WBP_OverHeadPosture.WBP_OverHeadPosture_C"))
      (bind _output_get_4 (Variables|Default|SetPostureBarWidget _returnvalue_4))
      (UserInterface|SetWidget (Variables|Default|GetPosturebarComponent) _output_get_4))
    (:then_2
      (bind _output_get_5 (Variables|Default|SetHealthComponent (Actor|GetComponentbyClass (Components|GetOwner) "/Game/MainContent/Design/Player/SharedComponents/AC_HealthComponent.AC_HealthComponent_C")))
      (EventDispatchers|BindEventtoOnDamageTaken _output_get_5 (delegate Custom|UpdateHealthAndPosture))
      (EventDispatchers|BindEventtoOnDeath _output_get_5 (delegate Custom|UpdateHealthAndPosture))
      (EventDispatchers|BindEventtoOnStunEnd _output_get_5 (delegate Custom|UpdateHealthAndPosture)))))

(event EventTick
  (params (DeltaSeconds :type Float%20%28single-precision%29))
  (bind _posturebarcomponent (Variables|Default|GetPosturebarComponent))
  (bind _posturebarcomponent_2 (Variables|Default|GetPosturebarComponent))
  (bind _healthbarcomponent (Variables|Default|GetHealthbarComponent))
  (bind _playercamera (Variables|Default|GetPlayerCamera))
  (bind _returnvalue (Transformation|GetWorldRotation _healthbarcomponent))
  (bind _returnvalue_2 (Camera|GetCameraLocation _playercamera))
  (bind _returnvalue_3 (Transformation|GetWorldRotation _posturebarcomponent_2))
  (if (Rendering|IsVisible (Variables|Default|GetHealthbarComponent))
    (Transformation|SetWorldRotation _healthbarcomponent (Math|Rotator|MakeRotator (.roll _returnvalue) (.pitch _returnvalue) (.yaw (Math|Rotator|FindLookatRotation (Transformation|GetWorldLocation (Variables|Default|GetHealthbarComponent)) _returnvalue_2))) false false))
  (if (Rendering|IsVisible _posturebarcomponent)
    (Transformation|SetWorldRotation _posturebarcomponent_2 (Math|Rotator|MakeRotator (.roll _returnvalue_3) (.pitch _returnvalue_3) (.yaw (Math|Rotator|FindLookatRotation (Transformation|GetWorldLocation _posturebarcomponent) _returnvalue_2))) false false)))