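; Shared player combat component that runs targeted melee combo attacks and applies weapon hits.
; Attack sphere-traces ahead for an "Enemy" pawn, then motion-warps to it with either a long-range zip montage or a combo montage picked by a Chooser from combo data.
; HitDetection sphere-traces between weapon or body sockets, sending damage and posture damage to AC_HealthComponent, with a hit list preventing repeat hits per combo attack.
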(event Custom|Attack
  (params (AttackType :type Gameplay%20Tag%20Structure))
  (bind _returnvalue (Components|GetOwner))
  (bind _combodata (Variables|Default|GetComboData))
  (bind (_currentanim _attackexist_) (Utilities|Struct|BreakF_ComboData _combodata))
  (bind _returnvalue_2 (Transformation|GetActorRotation _returnvalue))
  (if (Variables|Default|GetCanAttack?)
    (Utilities|Struct|SetmembersinF_ComboData (Variables|Default|GetComboData) (GameplayTags|MakeGameplayTagContainerfromTag AttackType))
    (bind (_foundenemy _shouldzip) (CallFunction|DetectEnemy))
    (if (and _foundenemy _shouldzip)
      (CallFunction|SnaptoTarget)
      (elif _foundenemy
        (Utilities|FlowControl|Sequence
          (:then_0
            (Class|MotionWarpingComponent|AddorUpdateWarpTarget (Variables|Default|GetMotionWarping) (Utilities|Struct|MakeMotionWarpingTarget "AttackTarget" (- (Transformation|GetActorLocation (Variables|Default|GetTargetEnemy)) (* (Math|Vector|GetForwardVector _returnvalue_2) 5e+01)) _returnvalue_2 0 "None" false "0.000000,0.000000,0.000000" "0.000000,0.000000,0.000000")))
          (:then_1
            (bind _result (|EvaluateChooser2 _combodata)
              (:execute
                (if _attackexist_
                  (Utilities|Struct|SetmembersinF_ComboData _combodata _result)
                  (Animation|Montage|PlayMontage (Variables|Default|GetCharacterMesh) _currentanim
                    (:then
                      (Utilities|Array|Clear (Variables|Default|GetHitEnemies))
                      (Variables|Default|SetCanAttack? false))
                    (:OnCompleted
                      (Utilities|Struct|SetmembersinF_ComboData (Variables|Default|GetComboData) 0 "(GameplayTags=)")
                      (Variables|Default|SetCanAttack? true)))
                  (else
                    (Variables|Default|SetCanAttack? false)))))))))))

(event Custom|SnapToTarget
  (bind _returnvalue (Components|GetOwner))
  (bind _returnvalue_2 (Transformation|GetActorRotation _returnvalue))
  (Class|MotionWarpingComponent|AddorUpdateWarpTarget (Variables|Default|GetMotionWarping) (Utilities|Struct|MakeMotionWarpingTarget "AttackTarget" (- (Transformation|GetActorLocation (Variables|Default|GetTargetEnemy)) (* (Math|Vector|GetForwardVector _returnvalue_2) 1e+02)) _returnvalue_2 0 "None" false "0.000000,0.000000,0.000000" "0.000000,0.000000,0.000000"))
  (Animation|Montage|PlayMontage (Variables|Default|GetCharacterMesh) (Utilities|Struct|BreakF_Weapon (Variables|Default|GetWeapon%20Data))
    (:then
      (Variables|Default|SetCanAttack? false))
    (:OnCompleted
      (Variables|Default|SetCanAttack? true))))

(event Custom|SetWeapon
  (params (Weapon :type F%20Weapon%20Structure))
  (bind _output_get (Variables|Default|SetWeapon%20Data Weapon))
  (Utilities|Struct|SetmembersinF_ComboData (Variables|Default|GetComboData) (Utilities|Struct|BreakF_Weapon _output_get) 0))

(event EventBeginPlay
  (bind _returnvalue (Components|GetOwner))
  (Variables|Default|SetCharacterMesh (Actor|GetComponentbyClass _returnvalue "/Script/Engine.SkeletalMeshComponent"))
  (Variables|Default|SetMotionWarping (Actor|GetComponentbyClass _returnvalue "/Script/MotionWarping.MotionWarpingComponent"))
  (Variables|Default|SetCharacterMovement (Actor|GetComponentbyClass (Components|GetOwner) "/Script/Engine.CharacterMovementComponent")))

(fn DetectEnemy
  (bind _returnvalue (Components|GetOwner))
  (bind _charactermovement (Variables|Default|GetCharacterMovement))
  (bind _returnvalue_2 (Transformation|GetActorLocation _returnvalue))
  (bind _returnvalue_3 (Class|CharacterMovementComponent|GetLastUpdateRotation _charactermovement))
  (bind _returnvalue_4 (Math|Vector|GetForwardVector _returnvalue_3))
  (bind _returnvalue_5 (Math|Vector|Normalize _returnvalue_4))
  (bind (_outhit _returnvalue_6) (Collision|SphereTraceForObjects (+ _returnvalue_2 (* _returnvalue_5 5e+01)) (+ _returnvalue_2 (* _returnvalue_5 (Variables|Default|GetMaxEnemyDistance))) 5e+01 (Utilities|Array|MakeArray "ObjectTypeQuery3") false 0 "ForDuration" true "(R=1.000000,G=0.000000,B=0.000000,A=1.000000)" "(R=0.000000,G=1.000000,B=0.000000,A=1.000000)" 1.0))
  (if _returnvalue_6
    (if (Actor|ActorHasTag (Components|GetOwner (.HitComponent (Collision|BreakHitResult _outhit))) "Enemy")
      (Variables|Default|SetTargetEnemy (Components|GetOwner (.HitComponent (Collision|BreakHitResult _outhit))))
      (return true (> (.Distance (Collision|BreakHitResult _outhit)) (Variables|Default|GetMinimumZipDistance)))
      (else
        _)))
  (return false false))

(fn HitDetection
  (params (StartSocket :type Name) (EndSocket :type Name) (Radius :type Float%20%28double-precision%29))
  (bind _charactermesh (Variables|Default|GetCharacterMesh))
  (bind _charactermesh_2 (Variables|Default|GetCharacterMesh))
  (bind _attack_data (Variables|Default|GetAttack%20Data))
  (bind (_animation _damage _posturepower) (Utilities|Struct|BreakF_AttackData _attack_data))
  (bind _returnvalue (Components|GetChildComponent _charactermesh 0))
  (if (Utilities|Enum|Equal(Enum) (Utilities|Struct|BreakF_Weapon (Variables|Default|GetWeapon%20Data)) "NewEnumerator0")
    (LocalVariables|SetStartPoint (Transformation|GetSocketLocation _charactermesh_2 StartSocket))
    (LocalVariables|SetEndPoint (Transformation|GetSocketLocation _charactermesh_2 EndSocket))
    (else
      (LocalVariables|SetStartPoint (Transformation|GetSocketLocation _returnvalue StartSocket))
      (LocalVariables|SetEndPoint (Transformation|GetSocketLocation _returnvalue EndSocket))))
  (bind (_outhit _returnvalue_2) (Collision|SphereTraceForObjects (LocalVariables|GetStartPoint) (LocalVariables|GetEndPoint) Radius (Utilities|Array|MakeArray "ObjectTypeQuery3") false 0 "ForDuration" true "(R=1.000000,G=0.000000,B=0.000000,A=1.000000)" "(R=0.000000,G=1.000000,B=0.000000,A=1.000000)" 1.0))
  (if _returnvalue_2
    (if (== (Utilities|Array|FindItem (Variables|Default|GetHitEnemies) (.HitActor (Collision|BreakHitResult _outhit))) -1)
      (Default|TakeDamage (Actor|GetComponentbyClass (.HitActor (Collision|BreakHitResult _outhit)) "/Game/MainContent/Design/Player/SharedComponents/AC_HealthComponent.AC_HealthComponent_C") _damage _posturepower)
      (Utilities|Array|AddUnique (Variables|Default|GetHitEnemies) (.HitActor (Collision|BreakHitResult _outhit))))))