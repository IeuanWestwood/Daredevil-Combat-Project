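; Shared player actor component that tracks the current weapon and handles equipping picked-up weapons.
; InitHandler stores the weapon holder component and loads the current weapon's data from DT_Weapons.
; EquipWeapon queries the pickup through PickupWeaponMessage, looks up its table row, then swaps the holder's skeletal mesh and snaps it to the owner's weapon_r socket.
; UnequipWeapon, called before replacing an armed weapon, is an empty stub.
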(fn InitHandler
  (params (WeaponHolder :type Skeletal%20Mesh%20Component%20Object%20Reference))
  (Variables|Default|SetWeapon%20Holder WeaponHolder)
  (bind _returnvalue (Utilities|GetDataTableRow "/Game/MainContent/Design/Weapons/DT_Weapons.DT_Weapons" (.RowName (Utilities|Struct|BreakDataTableRowHandle (Variables|Default|GetCurrentWeaponRow))))
    (:then
      (Variables|Default|SetCurrentWeaponData _returnvalue))))

(fn EquipWeapon
  (params (NewWeapon :type Actor%20Object%20Reference))
  (bind _weapon_holder (Variables|Default|GetWeapon%20Holder))
  (bind (_canpickup _weapon) (Class|BPIPickupable|PickupWeapon(Message) NewWeapon))
  (if _canpickup
    (bind _output_get (LocalVariables|SetNewWeaponRow _weapon))
    (bind _returnvalue (Utilities|GetDataTableRow "/Game/MainContent/Design/Weapons/DT_Weapons.DT_Weapons" (.rowname _output_get))
      (:then
        (LocalVariables|SetNewWeaponData _returnvalue)
        (if (== (.RowName (Utilities|Struct|BreakDataTableRowHandle (Variables|Default|GetCurrentWeaponRow))) "Unarmed")
          _
          (else
            (CallFunction|UnequipWeapon)))
        (Variables|Default|SetCurrentWeaponRow (LocalVariables|GetNewWeaponRow))
        (bind _output_get_2 (Variables|Default|SetCurrentWeaponData (LocalVariables|GetNewWeaponData)))
        (Components|SkeletalMesh|SetSkeletalMeshAsset _weapon_holder (.WeaponSkeletalMesh (Utilities|Struct|BreakF_Weapon _output_get_2)))
        (Transformation|AttachComponentToComponent _weapon_holder (Actor|GetComponentbyClass (Components|GetOwner) "/Script/Engine.SkeletalMeshComponent") "weapon_r" "SnapToTarget" "SnapToTarget" "SnapToTarget" false))
      (:RowNotFound
        (return false)))
    (else
      (return false))))

(fn UnequipWeapon
  (return))