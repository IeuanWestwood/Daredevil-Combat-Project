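; BP_WeaponPickup is a weapon pickup that tracks whether a player is close enough to take it.
; Its construction script looks up the weapon's DT_Weapons row, sets the static mesh, sizes the sphere to PickupRange and offsets it along world X by half the mesh's Z extent.
; Sphere overlaps with Player-tagged actors toggle CanPickUp.
; PickupWeapon only returns that flag and the weapon, without granting or destroying anything.
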(event OnComponentBeginOverlap(Sphere)
  (params (OverlappedComponent :type Primitive%20Component%20Object%20Reference) (OtherActor :type Actor%20Object%20Reference) (OtherComp :type Primitive%20Component%20Object%20Reference) (OtherBodyIndex :type Integer) (bFromSweep :type Boolean) (SweepResult :type Hit%20Result%20Structure%20%28by%20ref%29))
  (if (Actor|ActorHasTag OtherActor "Player")
    (Variables|Default|SetCanPickUp? true)))

(event OnComponentEndOverlap(Sphere)
  (params (OverlappedComponent :type Primitive%20Component%20Object%20Reference) (OtherActor :type Actor%20Object%20Reference) (OtherComp :type Primitive%20Component%20Object%20Reference) (OtherBodyIndex :type Integer))
  (if (Actor|ActorHasTag OtherActor "Player")
    (Variables|Default|SetCanPickUp? false)))

(fn ConstructionScript
  (bind _returnvalue (Utilities|GetDataTableRow "/Game/MainContent/Design/Weapons/DT_Weapons.DT_Weapons" (.rowname (Variables|Default|GetWeapon)))
    (:then
      (bind _output_get (Variables|Default|SetWeaponData _returnvalue))
      (Components|StaticMesh|SetStaticMesh (Variables|Default|GetWeaponMesh) (.weaponstaticmesh _output_get))
      (Components|Sphere|SetSphereRadius (Variables|Default|GetSphere) (Variables|Default|GetPickupRange) true)
      (Transformation|AddWorldOffset (Variables|Default|GetSphere) (Math|Vector|MakeVector (/ (.z (.boxextent (StaticMesh|GetBounds (Variables|/Script/Engine.StaticMeshComponent|GetStaticMesh (Variables|Default|GetWeaponMesh))))) 2.0) 0.0 0.0) false false))))

(fn PickupWeapon
  (return (Variables|Default|GetCanPickUp?) (Variables|Default|GetWeapon)))